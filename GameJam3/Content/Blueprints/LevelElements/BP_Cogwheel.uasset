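; BP_Cogwheel is a collectible cog that counts toward the level's elevator.
; On BeginPlay it caches the first BP_Elevator it finds.
; Its sphere overlap with the player shows a WBP_TextPopup pickup prompt and sets Inrange; leaving removes all such popups and clears the flag.
; The Collected event, not triggered within this graph, calls IncreaseCollectCog on the elevator and destroys the cog.
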(event OnComponentBeginOverlap(Sphere)
  (params (OverlappedComponent :type Primitive%20Component%20Object%20Reference) (OtherActor :type Actor%20Object%20Reference) (OtherComp :type Primitive%20Component%20Object%20Reference) (OtherBodyIndex :type Integer) (bFromSweep :type Boolean) (SweepResult :type Hit%20Result%20Structure%20%28by%20ref%29))
  (if (== OtherActor (Game|GetPlayerCharacter 0))
    (bind _returnvalue (UserInterface|CreateWidget "/Game/Menu/HUD/WBP_TextPopup.WBP_TextPopup_C"))
    (Variables|/Game/Menu/HUD/WBP_TextPopup.WBP_TextPopup_C|SetText _returnvalue "Press E to pick up")
    (UserInterface|Viewport|AddtoViewport _returnvalue 0)
    (Variables|Default|SetbInrange true)))

(event OnComponentEndOverlap(Sphere)
  (params (OverlappedComponent :type Primitive%20Component%20Object%20Reference) (OtherActor :type Actor%20Object%20Reference) (OtherComp :type Primitive%20Component%20Object%20Reference) (OtherBodyIndex :type Integer))
  (if (== OtherActor (Game|GetPlayerCharacter 0))
    (bind _foundwidgets (Widget|GetAllWidgetsOfClass "/Game/Menu/HUD/WBP_TextPopup.WBP_TextPopup_C" false))
    (for _array_element _foundwidgets
      (Widget|RemovefromParent _array_element)
      (Variables|Default|SetbInrange false))))

(event Custom|Collected
  (Default|IncreaseCollectCog (Variables|Default|GetAs%20BP%20Elevator))
  (Actor|DestroyActor))

(event EventBeginPlay
  (bind _outactors (Actor|GetAllActorsOfClass "/Game/Blueprints/LevelElements/BP_Elevator.BP_Elevator_C"))
  (bind _asbp_elevator (Utilities|Casting|CastToBP_Elevator (Utilities|Array|Get(acopy) _outactors)))
  (Variables|Default|SetAs%20BP%20Elevator _asbp_elevator))

(event Collision|EventActorBeginOverlap
  (params (OtherActor :type Actor%20Object%20Reference)))

(fn ConstructionScript)