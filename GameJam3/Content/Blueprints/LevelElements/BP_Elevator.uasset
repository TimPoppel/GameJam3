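; Elevator level element that ends the level or game once the player has collected enough cogwheels.
; An external call to IncreaseCollectCog raises the count, capped at MaxCog.
; When the player enters the Box trigger, it calls the ending dispatcher if the count is met, otherwise shows a WBP_TextPopup stating how many cogwheels remain.
; Leaving the trigger removes all popups of that class.
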(event OnComponentBeginOverlap(Box)
  (params (OverlappedComponent :type Primitive%20Component%20Object%20Reference) (OtherActor :type Actor%20Object%20Reference) (OtherComp :type Primitive%20Component%20Object%20Reference) (OtherBodyIndex :type Integer) (bFromSweep :type Boolean) (SweepResult :type Hit%20Result%20Structure%20%28by%20ref%29))
  (bind _maxcog (Variables|Default|GetMaxCog))
  (bind _cogwheelcollected (Variables|Default|GetCogwheelCollected))
  (bind _returnvalue (- _maxcog _cogwheelcollected))
  (if (== OtherActor (Game|GetPlayerCharacter 0))
    (if (>= (Variables|Default|GetCogwheelCollected) (Variables|Default|GetMaxCog))
      (Default|CallEndingDispatcher)
      (else
        (bind _returnvalue_2 (UserInterface|CreateWidget "/Game/Menu/HUD/WBP_TextPopup.WBP_TextPopup_C"))
        (if (== _returnvalue 1)
          (Variables|/Game/Menu/HUD/WBP_TextPopup.WBP_TextPopup_C|SetText _returnvalue_2 "I need 1 more cogwheel.")
          (else
            (Variables|/Game/Menu/HUD/WBP_TextPopup.WBP_TextPopup_C|SetText _returnvalue_2 (Utilities|Text|ToText(String) (Utilities|String|Append "I still need " (Utilities|String|ToString(Integer) _returnvalue) " cogwheels.")))))
        (UserInterface|Viewport|AddtoViewport _returnvalue_2 0)))))

(event OnComponentEndOverlap(Box)
  (params (OverlappedComponent :type Primitive%20Component%20Object%20Reference) (OtherActor :type Actor%20Object%20Reference) (OtherComp :type Primitive%20Component%20Object%20Reference) (OtherBodyIndex :type Integer))
  (if (== OtherActor (Game|GetPlayerCharacter 0))
    (bind _foundwidgets (Widget|GetAllWidgetsOfClass "/Game/Menu/HUD/WBP_TextPopup.WBP_TextPopup_C" false))
    (for _array_element _foundwidgets
      (Widget|RemovefromParent (stale OnComponentBeginOverlap(Box) _returnvalue_2)))))

(event Custom|IncreaseCollectCog
  (Math|Integer|IncrementInt (Variables|Default|GetCogwheelCollected)
    (:%20%20
      (if (> (Variables|Default|GetCogwheelCollected) (Variables|Default|GetMaxCog))
        (Variables|Default|SetCogwheelCollected (Variables|Default|GetMaxCog))))))

(event EventBeginPlay
  (Variables|Default|SetCogwheelCollected 0))

(event Collision|EventActorBeginOverlap
  (params (OtherActor :type Actor%20Object%20Reference)))

(event EventTick
  (params (DeltaSeconds :type Float%20%28single-precision%29)))

(fn ConstructionScript)