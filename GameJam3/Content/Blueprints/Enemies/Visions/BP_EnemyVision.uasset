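; BP_EnemyVision is a temporary enemy vision actor with a Niagara-style effect and point light that removes itself.
; It self-destructs after LifeTime, or after ParticleDuration once SeeActor fires, clearing its Spawner's HasVision flag either way.
; SeeActor deactivates NSVision and starts a one-time looping timer setup, apparently driving DecreaseLight to step the light's intensity down linearly as the particles fade.
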(event Custom|SeeActor
  (Components|Activation|SetActive (Variables|Default|GetNS_Vision) false false)
  (Utilities|FlowControl|Sequence
    (:then_0
      (Utilities|FlowControl|DoOnce false
        (:Completed
          (Variables|Default|SetMaxIntensity (Variables|/Script/Engine.LightComponentBase|GetIntensity (Variables|Default|GetPointLight)))
          (bind _output_get (Variables|Default|SetIntensityStep (/ (Variables|Default|GetMaxIntensity) (/ (Variables|Default|GetParticleDuration) 0.1))))
          (Variables|Default|SetIntensityRemove _output_get)
          (Utilities|Time|SetTimerbyEvent (EventDispatchers|CreateEvent :!event Custom|DecreaseLight) 0.1 true))))
    (:then_1
      (Utilities|FlowControl|Delay (Variables|Default|GetParticleDuration))
      (Variables|/Game/Blueprints/Enemies/Visions/BP_VisionSpawnPoint.BP_VisionSpawnPoint_C|SetHasVision (Variables|Default|GetSpawner) false)
      (Actor|DestroyActor))))

(event Custom|DecreaseLight
  (Rendering|Components|Light|SetIntensity (Variables|Default|GetPointLight) (- (Variables|Default|GetMaxIntensity) (Variables|Default|GetIntensityRemove)))
  (Variables|Default|SetIntensityRemove (+ (Variables|Default|GetIntensityStep) (Variables|Default|GetIntensityRemove))))

(event EventBeginPlay
  (Utilities|FlowControl|Delay (Variables|Default|GetLifeTime))
  (Variables|/Game/Blueprints/Enemies/Visions/BP_VisionSpawnPoint.BP_VisionSpawnPoint_C|SetHasVision (Variables|Default|GetSpawner) false)
  (Actor|DestroyActor))

(fn ConstructionScript)