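; Aggressive enemy that hunts the player through a behavior tree, with movement and awareness driven by the player's insanity.
; Tick feeds player location and an insanity-based PlayerIsLit flag to the blackboard, scaling walk speed at high insanity.
; KillPlayer freezes the player, pulls the camera toward the enemy's light with post-processing and sound, then loads DeathLevel.
; Ending events halt and teleport the enemy or send it sprinting to EndGoal.
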(event Custom|Ending
  (Utilities|FlowControl|DoOnce false
    (:Completed
      (AI|Logic|StopLogic (Variables|Default|GetBehaviorTree) "")
      (Components|Movement|StopMovementImmediately (Variables|Character|GetCharacterMovement))
      (Transformation|SetActorLocation "-370.000000,-1450.000000,140.000000" false false))))

(event Custom|KillPlayer
  (bind _pointlight2 (Variables|Default|GetPointLight2))
  (bind _returnvalue (Transformation|GetWorldLocation _pointlight2))
  (Variables|Default|SetKillingPlayer true)
  (CallFunction|PlayDeathSound)
  (Variables|Death|SetLerpAlpha (Math|Float|Clamp(Float) (+ (Variables|Death|GetLerpAlpha) (Variables|Death|GetDeathSpeed))))
  (bind _asbp_player (Utilities|Casting|CastToBP_Player (Game|GetPlayerCharacter 0)))
  (Pawn|Components|CharacterMovement|DisableMovement (Variables|/Script/Engine.Character|GetCharacterMovement _asbp_player))
  (Input|SetInputModeUIOnly (Game|GetPlayerController 0) 0 "DoNotLock")
  (Transformation|SetWorldLocation (Variables|/Game/Blueprints/Character/BP_Player.BP_Player_C|GetCamera _asbp_player) (Math|Vector|Lerp(Vector) (Transformation|GetWorldLocation (Variables|/Game/Blueprints/Character/BP_Player.BP_Player_C|GetCamera _asbp_player)) _returnvalue (Variables|Death|GetLerpAlpha)) false false)
  (Variables|/Script/Engine.CameraComponent|SetbUsePawnControlRotation (Variables|/Game/Blueprints/Character/BP_Player.BP_Player_C|GetCamera _asbp_player) false)
  (Variables|/Script/Engine.CameraComponent|SetPostProcessSettings (Variables|/Game/Blueprints/Character/BP_Player.BP_Player_C|GetCamera _asbp_player) (Variables|Default|GetPost%20Process%20Settings))
  (Transformation|SetWorldRotation (Variables|/Game/Blueprints/Character/BP_Player.BP_Player_C|GetCamera _asbp_player) (Math|Rotator|Lerp(Rotator) (Transformation|GetWorldRotation (Variables|/Game/Blueprints/Character/BP_Player.BP_Player_C|GetCamera _asbp_player)) (Math|Rotator|FindLookatRotation (Transformation|GetWorldLocation (Variables|/Game/Blueprints/Character/BP_Player.BP_Player_C|GetCamera _asbp_player)) _returnvalue) (* (Variables|Death|GetLerpAlpha) 3.0)) false false)
  (Utilities|FlowControl|Delay 2.5)
  (Game|OpenLevel(byName) "DeathLevel"))

(event Custom|PlayDeathSound
  (Utilities|FlowControl|DoOnce false
    (:Completed
      (Audio|PlaySoundatLocation (Variables|Default|GetScarySound) (Transformation|GetActorLocation) "0, 0, 0" 1.0 1.0 0.0 0 0 0 0))))

(event Custom|EndingScene
  (bind _charactermovement (Variables|Character|GetCharacterMovement))
  (Variables|/Script/Engine.CharacterMovementComponent|SetMaxAcceleration _charactermovement 3e+03)
  (Variables|/Script/Engine.CharacterMovementComponent|SetMaxWalkSpeed _charactermovement 3e+03)
  (AI|Navigation|MovetoLocation (AI|GetAIController self) (Variables|Default|GetEndGoal) -1.0 true true false true 0))

(event EventBeginPlay
  (AI|Logic|StartLogic (Variables|Default|GetBehaviorTree))
  (AI|Components|Blackboard|SetValueasBool (Variables|Default|GetBlackboard) (Utilities|Name|MakeLiteralName "PlayerIsLit") true)
  (Variables|Default|SetMovementSpeed (Variables|/Script/Engine.CharacterMovementComponent|GetMaxWalkSpeed (Variables|Character|GetCharacterMovement))))

(event EventTick
  (params (DeltaSeconds :type Float%20%28single-precision%29))
  (bind _returnvalue (Game|GetPlayerCharacter 0))
  (bind _returnvalue_2 (Game|GetPlayerCharacter 0))
  (bind _asbp_player (Utilities|Casting|CastToBP_Player _returnvalue))
  (bind _asbp_player_2 (Utilities|Casting|CastToBP_Player _returnvalue_2))
  (bind _insanitylevel (Variables|/Game/Blueprints/Character/BP_Player.BP_Player_C|GetInsanityLevel _asbp_player_2))
  (bind _returnvalue_3 (== _insanitylevel 2))
  ;[1 1 1] Get Player Location
  (AI|Components|Blackboard|SetValueasVector (Variables|Default|GetBlackboard) (Utilities|Name|MakeLiteralName "PlayerLocation") (Transformation|GetWorldLocation (Variables|/Script/Engine.Character|GetCapsuleComponent (Game|GetPlayerCharacter 0))))
  (Utilities|FlowControl|Sequence
    (:then_0
      ;[1 1 1] Logic to make enemies chase even when technically impossible to reach
      (if (not (Variables|Default|GetKillingPlayer))
        (if _returnvalue_3
          (AI|Components|Blackboard|SetValueasBool (Variables|Default|GetBlackboard) (Utilities|Name|MakeLiteralName "PlayerIsLit") (not _returnvalue_3))
          (elif (< (Transformation|GetDistanceTo self _returnvalue_2) 9e+02)
            (AI|Components|Blackboard|SetValueasBool (Variables|Default|GetBlackboard) (Utilities|Name|MakeLiteralName "PlayerIsLit") (not _returnvalue_3))))))
    (:then_1
      (if (> (Variables|/Game/Blueprints/Character/BP_Player.BP_Player_C|GetInsanityLevel _asbp_player) 1)
        (Variables|/Script/Engine.CharacterMovementComponent|SetMaxWalkSpeed (Variables|Character|GetCharacterMovement) (* (Variables|Default|GetMovementSpeed) (/ (* (Variables|/Game/Blueprints/Character/BP_Player.BP_Player_C|GetInsanityAmount _asbp_player) 1.5) (Variables|/Game/Blueprints/Character/BP_Player.BP_Player_C|GetMaxInsanityAmount _asbp_player))))
        (else
          (Variables|/Script/Engine.CharacterMovementComponent|SetMaxWalkSpeed (Variables|Character|GetCharacterMovement) 8e+02))))))

(fn ConstructionScript)