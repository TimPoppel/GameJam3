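; Oil lamp component that toggles its owner's lamp, burns fuel and warns the player as it runs low.
; Looping timers drive fuel use, with an extra cost on each lighting.
; Exact fuel-percentage milestones swap the Niagara flame, play a cue, show a text popup and step both point lights toward lower intensity.
; It finds lights, flame and mesh on the owner by tag, toggling visibility and mesh shadow.
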(event Custom|ToggleLamp
  (bind _timerhandlecheck_ (Variables|Default|GetTimerHandleCheck%25))
  (Audio|PlaySound2D "/Game/Audio/SE/PC/Lantern_on-off_Cue.Lantern_on-off_Cue" 1.0 1.0 0.0 0 0)
  (if (Variables|Default|GetbOutOfFuel)
    ;[1 1 1] Feedback that lamp is out of fuel
    (Utilities|Text "I'm Out of Fuel")
    (else
      ;[1 1 1] Check If Lit
      (if (Variables|Default|GetIsLit)
        (Variables|Default|SetIsLit false)
        (else
          (Variables|Default|SetIsLit true)))
      (if (Variables|Default|GetIsLit)
        (if (not (Variables|Default|GetbOutOfFuel))
          ;[1 1 1] Lit the lamp
          (CallFunction|TurnonLight)
          (CallFunction|AddFuel (* (Variables|Default|GetLightUpAmount) -1.0))
          ;[1 1 1] Start Depleting Fuel
          (CallFunction|FuelChanged)
          (bind _returnvalue (Utilities|Time|SetTimerbyEvent (EventDispatchers|CreateEvent :!event Custom|DepleteFuel) (Variables|Default|GetDepleteTime) true))
          (Variables|Default|SetTimerHandleDeplete _returnvalue)
          (if (Utilities|Time|IsValidTimerHandle _timerhandlecheck_)
            (Utilities|Time|UnpauseTimerbyHandle _timerhandlecheck_)))
        (else
          ;[1 1 1] Unlit the lamp
          (CallFunction|TurnOffLight)
          ;[1 1 1] Pause FuelDepleting
          (Utilities|Time|PauseTimerbyHandle (Variables|Default|GetTimerHandleDeplete))
          (Utilities|Time|PauseTimerbyHandle (Variables|Default|GetTimerHandleCheck%25)))))))

(event Custom|DecreaseLight
  (bind _returnvalue (Components|GetOwner))
  (bind _returnvalue_2 (Components|GetOwner))
  (bind _returnvalue_3 (Actor|GetComponentsbyTag _returnvalue_2 "/Script/Engine.PointLightComponent" "Light"))
  (bind _returnvalue_4 (Actor|GetComponentsbyTag _returnvalue "/Script/Engine.PointLightComponent" "Light"))
  (bind _output (Utilities|Array|Get(acopy) _returnvalue_3))
  (bind _output_2 (Utilities|Array|Get(acopy) _returnvalue_4 1))
  ;[1 1 1] Dimlight
  (if (== (Variables|Default|GetCurrentLightIntensity0) (Variables|Default|GetNewLightIntesity0))
    _
    (else
      (Utilities|IsValid _output
        (:Is%20Valid
          (Rendering|Components|Light|SetIntensity _output (- (Variables|Default|GetCurrentLightIntensity0) (Variables|Default|GetDepleteLight0)))
          (Variables|Default|SetCurrentLightIntensity0 (- (Variables|Default|GetCurrentLightIntensity0) (Variables|Default|GetDepleteLight0)))))))
  (if (== (Variables|Default|GetCurrentLightIntensity1) (Variables|Default|GetNewLightIntesity1))
    (Utilities|Time|ClearandInvalidateTimerbyHandle (Variables|Default|GetTimerHandleDim))
    (else
      (Utilities|IsValid _output_2
        (:Is%20Valid
          (Rendering|Components|Light|SetIntensity _output_2 (- (Variables|Default|GetCurrentLightIntensity1) (Variables|Default|GetDepleteLight1)))
          (Variables|Default|SetCurrentLightIntensity1 (- (Variables|Default|GetCurrentLightIntensity1) (Variables|Default|GetDepleteLight1))))))))

(event Custom|DepleteFuel
  ;[1 1 1] Check if we are out of fuel
  (if (<= (Variables|Default|GetCurrentFuel) 0.0)
    (Variables|Default|SetbOutofFuel true)
    (CallFunction|TurnOffLight)
    (Variables|Default|SetIsLit false)
    (if (>= (Variables|Default|GetCurrentFuel) 2.0)
      (goto _label Reset)
      (else
        (Utilities|FlowControl|DoOnce false :!label _label
          (:Completed
            (Audio|PlaySound2D "/Game/Audio/SE/PC/Lantern_Going_out_Cue.Lantern_Going_out_Cue" 1.0 1.0 0.0 0 0)))))
    (else
      ;[1 1 1] Deplete Fuel Properly
      (if (<= (- (Variables|Default|GetCurrentFuel) (Variables|Default|GetDepleteAmount)) 0.0)
        (Variables|Default|SetCurrentFuel 0.0)
        (Variables|Default|SetbOutofFuel true)
        (CallFunction|TurnOffLight)
        (Variables|Default|SetIsLit false)
        (else
          (Variables|Default|SetCurrentFuel (- (Variables|Default|GetCurrentFuel) (Variables|Default|GetDepleteAmount)))
          (Variables|Default|SetbOutofFuel false))))))

(event Custom|CheckCurrentFuel%25
  ;[1 1 1] Fuel% Popup
  (Utilities|FlowControl|Sequence
    (:then_0
      (Utilities|FlowControl|DoOnce false :!label _label
        (:Completed
          (if (> (Variables|Default|GetCurrentFuel) (* (Variables|Default|GetMaxFuel) 0.75))
            (Utilities|SetFire "/Game/OldMines/Effects/NS_TorchFire_2.NS_TorchFire_2")
            (Utilities|SetLightIntensity 1e+02)
            (elif (Utilities|FualEqual% 5e+01)
              (Utilities|SetFire "/Game/OldMines/Effects/NS_TorchFire_3.NS_TorchFire_3")
              (Utilities|SetLightIntensity 5e+01)
              (Audio|PlaySound2D "/Game/Audio/SE/PC/Flame_Milestone_Cue.Flame_Milestone_Cue" 1.0 1.0 0.0 0 0)
              (Utilities|Text "I have about half the fuel left to use.")
              (elif (Utilities|FualEqual% 25.0)
                (Utilities|SetFire "/Game/OldMines/Effects/NS_TorchFire_4.NS_TorchFire_4")
                (Utilities|SetLightIntensity 25.0)
                (Audio|PlaySound2D "/Game/Audio/SE/PC/Flame_Milestone_Cue.Flame_Milestone_Cue" 1.0 1.0 0.0 0 0)
                (Utilities|Text "Oh no I only have about a quarter of the fuel left.")
                (elif (Utilities|FualEqual% 1e+01)
                  (Utilities|SetFire "/Game/OldMines/Effects/NS_TorchFire_5.NS_TorchFire_5")
                  (Utilities|SetLightIntensity 1e+01)
                  (Audio|PlaySound2D "/Game/Audio/SE/PC/Flame_Milestone_Cue.Flame_Milestone_Cue" 1.0 1.0 0.0 0 0)
                  (Utilities|Text "Oh god only a small bit of fuel left.")
                  (elif (Utilities|FualEqual% 5.0)
                    (Utilities|SetFire "/Game/OldMines/Effects/NS_TorchFire_6.NS_TorchFire_6")
                    (Utilities|SetLightIntensity 5.0)
                    (Audio|PlaySound2D "/Game/Audio/SE/PC/Flame_Milestone_Cue.Flame_Milestone_Cue" 1.0 1.0 0.0 0 0)
                    (Utilities|Text "This flame won't last long, I should refill!")))))))))
    (:then_1
      (Utilities|FlowControl|Delay 1.0)
      (goto _label Reset))))

(event Custom|AddFuel
  (params (Amount :type Float%20%28double-precision%29))
  ;[1 1 1] Add Fuel Event
  (Variables|Default|SetCurrentFuel (+ Amount (Variables|Default|GetCurrentFuel)))
  (Variables|Default|SetbOutofFuel false)
  (if (> (Variables|Default|GetCurrentFuel) (Variables|Default|GetMaxFuel))
    (Variables|Default|SetCurrentFuel (Variables|Default|GetMaxFuel))
    (elif (< (Variables|Default|GetCurrentFuel) 0.0)
      (Variables|Default|SetCurrentFuel 0.0)
      (Variables|Default|SetbOutofFuel true))))

(event Custom|FuelChanged
  ;[1 1 1] Fuel% Popup
  (if (> (Variables|Default|GetCurrentFuel) (* (Variables|Default|GetMaxFuel) 0.75))
    (Utilities|SetFire "/Game/OldMines/Effects/NS_TorchFire_2.NS_TorchFire_2")
    (Utilities|SetLightIntensity 1e+02)
    (elif (Utilities|FualEqual% 5e+01)
      (Utilities|SetFire "/Game/OldMines/Effects/NS_TorchFire_3.NS_TorchFire_3")
      (Utilities|SetLightIntensity 5e+01)
      (Audio|PlaySound2D "/Game/Audio/SE/PC/Flame_Milestone_Cue.Flame_Milestone_Cue" 1.0 1.0 0.0 0 0)
      (Utilities|Text "I have about half the fuel left to use.")
      (elif (Utilities|FualEqual% 25.0)
        (Utilities|SetFire "/Game/OldMines/Effects/NS_TorchFire_4.NS_TorchFire_4")
        (Utilities|SetLightIntensity 25.0)
        (Audio|PlaySound2D "/Game/Audio/SE/PC/Flame_Milestone_Cue.Flame_Milestone_Cue" 1.0 1.0 0.0 0 0)
        (Utilities|Text "Oh no I only have about a quarter of the fuel left.")
        (elif (Utilities|FualEqual% 1e+01)
          (Utilities|SetFire "/Game/OldMines/Effects/NS_TorchFire_5.NS_TorchFire_5")
          (Utilities|SetLightIntensity 1e+01)
          (Audio|PlaySound2D "/Game/Audio/SE/PC/Flame_Milestone_Cue.Flame_Milestone_Cue" 1.0 1.0 0.0 0 0)
          (Utilities|Text "Oh god only a small bit of fuel left.")
          (elif (Utilities|FualEqual% 5.0)
            (Utilities|SetFire "/Game/OldMines/Effects/NS_TorchFire_6.NS_TorchFire_6")
            (Utilities|SetLightIntensity 5.0)
            (Audio|PlaySound2D "/Game/Audio/SE/PC/Flame_Milestone_Cue.Flame_Milestone_Cue" 1.0 1.0 0.0 0 0)
            (Utilities|Text "This flame won't last long, I should refill!")))))))

(event EventBeginPlay
  (bind _returnvalue (Components|GetOwner))
  (bind _returnvalue_2 (Actor|GetComponentsbyTag _returnvalue "/Script/Engine.PointLightComponent" "Light"))
  (bind _output (Utilities|Array|Get(acopy) _returnvalue_2))
  (bind _output_2 (Utilities|Array|Get(acopy) _returnvalue_2 1))
  (Variables|Default|SetCurrentFuel (Variables|Default|GetMaxFuel))
  (CallFunction|TurnOffLight)
  (Variables|Default|SetIsLit false)
  (bind _returnvalue_3 (Utilities|Time|SetTimerbyEvent (EventDispatchers|CreateEvent :!event Custom|CheckCurrentFuel%25) (Variables|Default|GetDepleteTime) true))
  (Variables|Default|SetTimerHandleCheck%25 _returnvalue_3)
  (Utilities|IsValid _output
    (:Is%20Valid
      (bind _output_get (Variables|Default|SetMaxLightIntensity0 (Variables|/Script/Engine.LightComponentBase|GetIntensity _output)))
      (Variables|Default|SetCurrentLightIntensity0 _output_get)
      (Utilities|IsValid _output_2
        (:Is%20Valid
          (bind _output_get_2 (Variables|Default|SetMaxLightIntensity1 (Variables|/Script/Engine.LightComponentBase|GetIntensity _output_2)))
          (Variables|Default|SetCurrentLightIntensity1 _output_get_2))))))

(fn TurnonLight
  (bind _returnvalue (Components|GetOwner))
  (bind _returnvalue_2 (Components|GetOwner))
  (bind _returnvalue_3 (Actor|GetComponentsbyTag _returnvalue "/Script/Engine.StaticMeshComponent" "Lamp"))
  (bind _returnvalue_4 (Actor|GetComponentsbyTag _returnvalue_2 "/Script/Engine.PointLightComponent" "Light"))
  (bind _output (Utilities|Array|Get(acopy) _returnvalue_3))
  (bind _output_2 (Utilities|Array|Get(acopy) _returnvalue_4))
  (Utilities|IsValid _output_2
    (:Is%20Valid
      (Utilities|IsValid (Utilities|Array|Get(acopy) _returnvalue_4 1)
        (:Is%20Valid
          (Utilities|IsValid (Utilities|Array|Get(acopy) (Actor|GetComponentsbyTag _returnvalue_2 "/Script/Niagara.NiagaraComponent" "Fire"))
            (:Is%20Valid
              (Rendering|SetVisibility _output_2 true false)
              (Utilities|IsValid _output
                (:Is%20Valid
                  (Rendering|SetCastShadow _output false))))))))))

(fn TurnOffLight
  (bind _returnvalue (Components|GetOwner))
  (bind _returnvalue_2 (Components|GetOwner))
  (bind _returnvalue_3 (Actor|GetComponentsbyTag _returnvalue "/Script/Engine.PointLightComponent" "Light"))
  (bind _returnvalue_4 (Actor|GetComponentsbyTag _returnvalue_2 "/Script/Engine.StaticMeshComponent" "Lamp"))
  (bind _output (Utilities|Array|Get(acopy) _returnvalue_3))
  (bind _output_2 (Utilities|Array|Get(acopy) _returnvalue_4))
  (Utilities|IsValid _output
    (:Is%20Valid
      (Utilities|IsValid (Utilities|Array|Get(acopy) _returnvalue_3 1)
        (:Is%20Valid
          (Utilities|IsValid (Utilities|Array|Get(acopy) (Actor|GetComponentsbyTag _returnvalue "/Script/Niagara.NiagaraComponent" "Fire"))
            (:Is%20Valid
              (Rendering|SetVisibility _output false false)
              (Utilities|IsValid _output_2
                (:Is%20Valid
                  (Rendering|SetCastShadow _output_2 true))))))))))