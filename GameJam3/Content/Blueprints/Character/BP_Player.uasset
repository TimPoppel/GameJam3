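; Player character with movement, clamped upward look, speed-scaled camera-shake bobbing, an oil lamp toggle and a pause menu.
; Timers drive sprint stamina drain and delayed refill, while Tick maps stamina steps to camera post-process presets and switches Walk/Run components from movement input.
; Pawn sensing notifies seen enemy visions.
; SpawnVisionNearby spawns a random vision at the nearest spawn point within a distance band.
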(event OnSeePawn(PawnSensing)
  (params (Pawn :type Pawn%20Object%20Reference))
  ;[1 1 1] See Visions
  (bind _asbp_enemy_vision (Utilities|Casting|CastToBP_EnemyVision Pawn))
  (Default|SeeActor _asbp_enemy_vision))

(event Custom|DrainStamina
  ;[1 1 1] Fatigue
  (if (>= (- (Variables|Sprint|GetStamina) (Variables|Sprint|GetFatigueStep)) 0.0)
    (Variables|Sprint|SetStamina (- (Variables|Sprint|GetStamina) (Variables|Sprint|GetFatigueStep)))
    (else
      (Variables|Sprint|SetbSprinting false)
      (Variables|/Script/Engine.CharacterMovementComponent|SetMaxWalkSpeed (Variables|Character|GetCharacterMovement) (Variables|Default|GetMaxWalkSpeed))
      (CallFunction|RefillStamina)
      (Variables|Default|SetStaminaCanFill true))))

(event Custom|RefillStamina
  ;[1 1 1] Refill Stamina
  (Utilities|FlowControl|RetriggerableDelay (Variables|Sprint|GetStaminaRefillDelay))
  (if (Variables|Default|GetStaminaCanFill)
    (Utilities|Time|SetTimerbyEvent (EventDispatchers|CreateEvent :!event Custom|StaminaFill) 0.1 true)))

(event Custom|StaminaFill
  ;[1 1 1] Refill Stamina
  (if (<= (+ (Variables|Sprint|GetStamina) (Variables|Sprint|GetFatigueStep)) (Variables|Sprint|GetMaxStamina))
    (Variables|Sprint|SetStamina (+ (Variables|Sprint|GetStamina) (Variables|Sprint|GetFatigueStep)))
    (else
      (Utilities|Time|SetTimerbyEvent (EventDispatchers|CreateEvent :!event Custom|StaminaFill) 0.0)
      (Audio|PlaySound2D "/Game/Audio/SE/PC/Breathing_in_Cue.Breathing_in_Cue" 1.0 1.0 0.0 0 0))))

(event Custom|SpawnVisionNearby
  ;[1 1 1] Spawn Visions
  (Variables|Visions|SetShortestDistance 999999999.0)
  (bind _outactors (Actor|GetAllActorsOfClass "/Game/Blueprints/Enemies/Visions/BP_VisionSpawnPoint.BP_VisionSpawnPoint_C"))
  (for _array_element _outactors
    (if (Math|Float|InRange(Float) (Transformation|GetDistanceTo _array_element self) (Variables|Visions|GetMinVisionDistance) (Variables|Visions|GetMaxVisionDistance))
      (Utilities|Map|Add (Variables|Visions|GetInRangeSpawners) _array_element (Transformation|GetDistanceTo _array_element self))))
  (bind _keys (Utilities|Map|Keys (Variables|Visions|GetInRangeSpawners)))
  (for _array_element_2 _keys
    (if (< (.Value (Utilities|Map|Find (Variables|Visions|GetInRangeSpawners) _array_element_2)) (Variables|Visions|GetShortestDistance))
      (Variables|Visions|SetShortestDistance (.Value (Utilities|Map|Find (Variables|Visions|GetInRangeSpawners) _array_element_2)))
      (Variables|Visions|SetNearestSpawner _array_element_2)))
  (Default|SpawnVision (Variables|Visions|GetNearestSpawner) (.OutItem (Utilities|Array|Random (Variables|Visions|GetVisions))))
  (Utilities|Map|Clear (Variables|Visions|GetInRangeSpawners)))

(event EventBeginPlay
  (Variables|Default|SetMaxWalkSpeed (Variables|/Script/Engine.CharacterMovementComponent|GetMaxWalkSpeed (Variables|Character|GetCharacterMovement)))
  (Variables|Default|SetMaxAcceleration (Variables|/Script/Engine.CharacterMovementComponent|GetMaxAcceleration (Variables|Character|GetCharacterMovement)))
  (Variables|Sprint|SetStamina (Variables|Sprint|GetMaxStamina)))

(event EventTick
  (params (DeltaSeconds :type Float%20%28single-precision%29))
  (bind _camera (Variables|Default|GetCamera))
  ;[1 1 1] Uggo but works
  (Utilities|FlowControl|Sequence
    (:then_0
      (switch int (Math|Float|Round (/ (Variables|Sprint|GetStamina) (Variables|Sprint|GetFatigueStep)))
        (:1
          (Variables|/Script/Engine.CameraComponent|SetPostProcessSettings _camera (Variables|PPS|GetPost%20Process%20Settings)))
        (:2
          (Variables|/Script/Engine.CameraComponent|SetPostProcessSettings _camera (Variables|PPS|GetPost%20Process%20Settings_0)))
        (:3
          (Variables|/Script/Engine.CameraComponent|SetPostProcessSettings _camera (Variables|PPS|GetPost%20Process%20Settings_1)))
        (:4
          (Variables|/Script/Engine.CameraComponent|SetPostProcessSettings _camera (Variables|PPS|GetPost%20Process%20Settings_2)))
        (:5
          (Variables|/Script/Engine.CameraComponent|SetPostProcessSettings _camera (Variables|PPS|GetPost%20Process%20Settings_3)))
        (:6
          (Variables|/Script/Engine.CameraComponent|SetPostProcessSettings _camera (Variables|PPS|GetPost%20Process%20Settings_4)))
        (:7
          (Variables|/Script/Engine.CameraComponent|SetPostProcessSettings _camera (Variables|PPS|GetPost%20Process%20Settings_5)))
        (:8
          (Variables|/Script/Engine.CameraComponent|SetPostProcessSettings _camera (Variables|PPS|GetPost%20Process%20Settings_6)))
        (:9
          (Variables|/Script/Engine.CameraComponent|SetPostProcessSettings _camera (Variables|PPS|GetPost%20Process%20Settings_7)))
        (:10
          (Variables|/Script/Engine.CameraComponent|SetPostProcessSettings _camera (Variables|PPS|GetPost%20Process%20Settings_8)))
        (:11
          (Variables|/Script/Engine.CameraComponent|SetPostProcessSettings _camera (Variables|PPS|GetPost%20Process%20Settings_9)))))
    (:then_1
      (if (== (+ (Input|AxisValues|GetMoveForward) (Input|AxisValues|GetMoveRight)) 0.0)
        (Audio|Components|Audio|Stop (Variables|Default|GetWalk))
        (elif (Variables|Sprint|GetbSprinting)
          (Components|Activation|Activate (Variables|Default|GetRun) false)
          (Audio|Components|Audio|Stop (Variables|Default|GetWalk))
          (else
            (Components|Activation|Activate (Variables|Default|GetWalk) false)
            (Audio|Components|Audio|Stop (Variables|Default|GetRun))))))))

(event Input|ActionEvents|InputActionToggleLamp
  (params (Key :type Key%20Structure :default "None"))
  (:Pressed
    (Default|ToggleLamp (Variables|Default|GetBP_Oillamp_Component))))

(event Input|ActionEvents|InputActionSprint
  (params (Key :type Key%20Structure :default "None"))
  ;[1 1 1] Sprint
  (:Pressed
    (if (> (Variables|Sprint|GetStamina) 0.0)
      (Variables|Default|SetStaminaCanFill false)
      (Utilities|Time|SetTimerbyEvent (EventDispatchers|CreateEvent :!event Custom|StaminaFill) 0.0)
      (Variables|Sprint|SetbSprinting true)
      (Variables|/Script/Engine.CharacterMovementComponent|SetMaxWalkSpeed (Variables|Character|GetCharacterMovement) (Variables|Sprint|GetSprintSpeed))
      (Utilities|Time|SetTimerbyEvent (EventDispatchers|CreateEvent :!event Custom|DrainStamina) 0.1 true)))
  (:Released
    (Variables|Sprint|SetbSprinting false)
    (Variables|/Script/Engine.CharacterMovementComponent|SetMaxWalkSpeed (Variables|Character|GetCharacterMovement) (Variables|Default|GetMaxWalkSpeed))
    (Utilities|Time|SetTimerbyEvent (EventDispatchers|CreateEvent :!event Custom|DrainStamina) 0.0)
    (CallFunction|RefillStamina)
    (Variables|Default|SetStaminaCanFill true)))

(event Input|ActionEvents|InputActionOpenPauseMenu
  (params (Key :type Key%20Structure :default "None"))
  (bind _returnvalue (Game|GetPlayerController 0))
  ;[1 1 1] Opening and closing Pause Menu with "P" and "Escape" key
  (:Pressed
    (Utilities|IsValid (Variables|Default|GetPauseMenuREF)
      (:Is%20Valid
        _)
      (:Is%20Not%20Valid
        (bind _returnvalue_2 (Game|ConstructObjectfromClass "/Game/Menu/Pause_Menu/Pause_Menu_Widget.Pause_Menu_Widget_C"))
        (Variables|Default|SetPauseMenuREF _returnvalue_2)))
    (if (Game|IsGamePaused)
      (Widget|RemovefromParent (Variables|Default|GetPauseMenuREF))
      (Game|SetGamePaused false)
      (Variables|/Script/Engine.PlayerController|SetbShowMouseCursor _returnvalue false)
      (Input|SetInputModeGameOnly _returnvalue)
      (else
        (UserInterface|Viewport|AddtoViewport (Variables|Default|GetPauseMenuREF) 0)
        (Game|SetGamePaused true)
        (Variables|/Script/Engine.PlayerController|SetbShowMouseCursor _returnvalue true)
        (Input|SetInputModeGameandUI _returnvalue (Variables|Default|GetPauseMenuREF) "LockInFullscreen" false)))))

(event Input|AxisEvents|InputAxisMoveForward
  (params (AxisValue :type Float%20%28single-precision%29))
  ;[1 1 1] Movement
  (Pawn|Input|AddMovementInput (Transformation|GetActorForwardVector) AxisValue false)
  ;[1 1 1] Bobbing
  (if (Variables|Camera|GetbBobbingEnabled)
    (if (Variables|Sprint|GetbSprinting)
      (Game|Feedback|ClientStartCameraShake (Game|GetPlayerController 0) "/Game/Blueprints/Character/BP_BobbingSprint.BP_BobbingSprint_C" (/ (Math|Vector|VectorLength (Transformation|GetVelocity)) (Variables|Camera|GetCameraShakeIntensity)) "CameraLocal" "0, 0, 0")
      (else
        (Game|Feedback|ClientStartCameraShake (Game|GetPlayerController 0) "/Game/Blueprints/Character/BP_BobbingWalk.BP_BobbingWalk_C" (/ (Math|Vector|VectorLength (Transformation|GetVelocity)) (Variables|Camera|GetCameraShakeIntensity)) "CameraLocal" "0, 0, 0")))))

(event Input|AxisEvents|InputAxisMoveRight
  (params (AxisValue :type Float%20%28single-precision%29))
  ;[1 1 1] Movement
  (Pawn|Input|AddMovementInput (Transformation|GetActorRightVector) AxisValue false)
  ;[1 1 1] Bobbing
  (if (Variables|Camera|GetbBobbingEnabled)
    (if (Variables|Sprint|GetbSprinting)
      (Game|Feedback|ClientStartCameraShake (Game|GetPlayerController 0) "/Game/Blueprints/Character/BP_BobbingSprint.BP_BobbingSprint_C" (/ (Math|Vector|VectorLength (Transformation|GetVelocity)) (Variables|Camera|GetCameraShakeIntensity)) "CameraLocal" "0, 0, 0")
      (else
        (Game|Feedback|ClientStartCameraShake (Game|GetPlayerController 0) "/Game/Blueprints/Character/BP_BobbingWalk.BP_BobbingWalk_C" (/ (Math|Vector|VectorLength (Transformation|GetVelocity)) (Variables|Camera|GetCameraShakeIntensity)) "CameraLocal" "0, 0, 0")))))

(event Input|AxisEvents|InputAxisLookUp
  (params (AxisValue :type Float%20%28single-precision%29))
  ;[1 1 1] Camera Rotation
  (bind _output_get (Variables|Camera|SetLookUp AxisValue))
  (if (> _output_get 0.0)
    (Pawn|Input|AddControllerPitchInput (Variables|Camera|GetLookUp))
    (elif (< (.pitch (Transformation|GetWorldRotation (Variables|Default|GetCamera))) (Variables|Camera|GetMaximumLookUp))
      (Pawn|Input|AddControllerPitchInput (Variables|Camera|GetLookUp)))))

(event Input|AxisEvents|InputAxisTurn
  (params (AxisValue :type Float%20%28single-precision%29))
  ;[1 1 1] Camera Rotation
  (Pawn|Input|AddControllerYawInput AxisValue))

(fn ConstructionScript)